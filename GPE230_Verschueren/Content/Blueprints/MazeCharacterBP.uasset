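; MazeCharacterBP is the maze character Blueprint, adding an input-triggered area stun against NPCs.
; Pressing Stun when the cooldown has expired resets it, activates the stun particle system and runs a zero-length multi-sphere object trace at the character's location.
; Each hit NPCAI receives Stunned, along with a leftover-looking debug print.
; Tick counts the cooldown down.
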(event `self.ReceiveTick`
  (params (DeltaSeconds :type "Float (single-precision)"))
  (if (> (`self.Stun Cooldown`) 0.0)
    (set `self.Stun Cooldown` (- (`self.Stun Cooldown`) DeltaSeconds))))

(event `InputAction|Stun`
  (params (Key :type "Key Structure"))
  (bind _returnvalue (`self.K2_GetActorLocation`))
  (:`Pressed`
    (if (<= (`self.Stun Cooldown`) 0.0)
      (set `self.Stun Cooldown` (`self.TimeBetweenStuns`))
      (`self.ActivateStunParticleSystem`)
      (bind _outhits (`KismetSystemLibrary.SphereTraceMultiForObjects` _returnvalue _returnvalue (`self.StunTraceRadius`) (`self.Stun Trace Types`)))
      (for _array_element _outhits
        (bind _asnpcai (cast `/Game/Blueprints/NPCAI` (`.HitActor` (`GameplayStatics.BreakHitResult` _array_element))))
        (`/Game/Blueprints/NPCAI.Stunned` _asnpcai)
        (`KismetSystemLibrary.PrintString` "why you bully me")))))

(fn `UserConstructionScript`)