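; AI controller for enemy NPCs that runs the NPCEnemyBT behavior tree and feeds its blackboard.
; On BeginPlay it stores the pawn's starting location as GuardPosition.
; Perception updates set TargetActor to a sensed actor and clear it when sensing fails.
; While a target is valid, Tick writes its distance to the pawn as DistanceToPlayer and prints that value on screen.
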(event `self.ReceiveBeginPlay`
  (`self.RunBehaviorTree` "/Game/Blueprints/NPCEnemyBT.NPCEnemyBT")
  (`BlackboardComponent.SetValueAsVector` (`AIBlueprintHelperLibrary.GetBlackboard` null) "GuardPosition" (`self.K2_GetActorLocation` (`self.K2_GetPawn`))))

(event `self.AIPerception.OnTargetPerceptionUpdated`
  (params (Actor :type "Actor Object Reference") (Stimulus :type "AIStimulus Structure"))
  (bind _returnvalue (`AIBlueprintHelperLibrary.GetBlackboard` null))
  (if (`.bSuccessfullySensed` (break `AIStimulus` Stimulus))
    (`BlackboardComponent.SetValueAsObject` _returnvalue "TargetActor" Actor)
    (else
      (`BlackboardComponent.SetValueAsObject` _returnvalue "TargetActor" null))))

(event `self.ReceiveTick`
  (params (DeltaSeconds :type "Float (single-precision)"))
  (bind _returnvalue (`BlackboardComponent.GetValueAsObject` (`AIBlueprintHelperLibrary.GetBlackboard` null) "TargetActor"))
  (if (`KismetSystemLibrary.IsValid` _returnvalue)
    (bind _asactor (cast `Actor` _returnvalue))
    (bind _returnvalue_2 (`self.GetDistanceTo` _asactor (`self.K2_GetPawn`)))
    (`BlackboardComponent.SetValueAsFloat` (`AIBlueprintHelperLibrary.GetBlackboard` null) "DistanceToPlayer" _returnvalue_2)
    (`KismetSystemLibrary.PrintString` (`KismetStringLibrary.Conv_DoubleToString` _returnvalue_2) true false (struct :`G` 0.66 :`B` 1.0 :`A` 1.0) 0.5)))

(fn `UserConstructionScript`)